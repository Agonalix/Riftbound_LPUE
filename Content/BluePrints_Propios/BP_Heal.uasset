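; BP_Heal is a temporary healing zone actor that heals BP_Player while the gate tied to its Sphere overlap is open.
; Tick drives two Delay-throttled branches: one counts LifeTime down each second and destroys the actor at zero, the other pulses every TickRATE into the gate.
; Sphere overlap begin and end open and close that gate, whose exit calls Heal on the overlapping player and prints its current HP.
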(event OnComponentBeginOverlap(Sphere)
  (params (OverlappedComponent :type Primitive%20Component%20Object%20Reference) (OtherActor :type Actor%20Object%20Reference) (OtherComp :type Primitive%20Component%20Object%20Reference) (OtherBodyIndex :type Integer) (bFromSweep :type Boolean) (SweepResult :type Hit%20Result%20Structure%20%28by%20ref%29))
  (Variables|Default|SetEnZona true)
  (Utilities|FlowControl|Gate true) ; enters at Open
)

(event OnComponentEndOverlap(Sphere)
  (params (OverlappedComponent :type Primitive%20Component%20Object%20Reference) (OtherActor :type Actor%20Object%20Reference) (OtherComp :type Primitive%20Component%20Object%20Reference) (OtherBodyIndex :type Integer))
  (Variables|Default|SetEnZona false)
  (Utilities|FlowControl|Gate true) ; enters at Close
)

(event EventBeginPlay)

(event Collision|EventActorBeginOverlap
  (params (OtherActor :type Actor%20Object%20Reference)))

(event EventTick
  (params (DeltaSeconds :type Float%20%28single-precision%29))
  (Utilities|FlowControl|Sequence
    (:then_0
      (Utilities|FlowControl|Delay 1.0)
      (bind _output_get (Variables|Default|SetLifeTime (- (Variables|Default|GetLifeTime) 1.0)))
      (if (<= _output_get 0.0)
        (Actor|DestroyActor)))
    (:then_1
      (Utilities|FlowControl|Delay (Variables|Default|GetTickRATE))
      (Utilities|FlowControl|Gate true
        (:Exit
          (bind _asbp_player (Utilities|Casting|CastToBP_Player (stale OnComponentBeginOverlap(Sphere) OtherActor)))
          (Default|Heal _asbp_player)
          (Development|PrintString (Utilities|String|ToString(Float) (Variables|/Game/BluePrints_Propios/BP_Player.BP_Player_C|GetHP%20current _asbp_player))))))))

(fn ConstructionScript)