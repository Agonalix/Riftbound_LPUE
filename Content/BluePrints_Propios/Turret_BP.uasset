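; Turret actor that repeatedly fires Bullet_T_BP from its own transform.
; Tick runs a FireRate Delay into CannonShoot, where a DoN caps shots at NShoot until the Reaload event resets it.
; Sphere1 overlaps set BP_Player's EnZona flag and open or close a Gate, but the Gate's exit drives nothing, so firing ignores player proximity.
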(event OnComponentBeginOverlap(Sphere1)
  (params (OverlappedComponent :type Primitive%20Component%20Object%20Reference) (OtherActor :type Actor%20Object%20Reference) (OtherComp :type Primitive%20Component%20Object%20Reference) (OtherBodyIndex :type Integer) (bFromSweep :type Boolean) (SweepResult :type Hit%20Result%20Structure%20%28by%20ref%29))
  (bind _asbp_player (Utilities|Casting|CastToBP_Player OtherActor))
  (Variables|/Game/BluePrints_Propios/BP_Player.BP_Player_C|SetEnZona _asbp_player true)
  (Utilities|FlowControl|Gate true) ; enters at Open
)

(event OnComponentEndOverlap(Sphere1)
  (params (OverlappedComponent :type Primitive%20Component%20Object%20Reference) (OtherActor :type Actor%20Object%20Reference) (OtherComp :type Primitive%20Component%20Object%20Reference) (OtherBodyIndex :type Integer))
  (bind _asbp_player (Utilities|Casting|CastToBP_Player OtherActor))
  (Variables|/Game/BluePrints_Propios/BP_Player.BP_Player_C|SetEnZona _asbp_player false)
  (Utilities|FlowControl|Gate true) ; enters at Close
)

(event Custom|CannonShoot
  (Utilities|FlowControl|DoN (Variables|Default|GetNShoot)
    (:Exit
      (Game|SpawnActorfromClass "/Game/BluePrints_Propios/Bullet_T_BP.Bullet_T_BP_C" (Transformation|GetActorTransform) "Undefined" "MultiplyWithRoot" 0 0))))

(event Custom|Reaload
  (Utilities|FlowControl|DoN (Variables|Default|GetNShoot)) ; enters at Reset
)

(event EventBeginPlay)

(event Collision|EventActorBeginOverlap
  (params (OtherActor :type Actor%20Object%20Reference)))

(event EventTick
  (params (DeltaSeconds :type Float%20%28single-precision%29))
  (Utilities|FlowControl|Sequence
    (:then_0
      (Utilities|FlowControl|Delay (Variables|Default|GetFireRate))
      (CallFunction|CannonShoot))
    (:then_1
      (Utilities|FlowControl|Gate true))))

(fn ConstructionScript)