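; BP_Spawner is an actor that repeatedly spawns BP_Pinches and BP_Heal actors near itself.
; A Delay on Tick throttles spawning to about one actor every two seconds.
; A looping random MultiGate picks the class, using both in random order before repeating.
; Each spawn lands at the spawner's height, randomly offset only along positive world X and Y, with default rotation and scale.
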(event EventTick
  (params (DeltaSeconds :type Float%20%28single-precision%29))
  (Utilities|FlowControl|Delay 2.0)
  (Utilities|FlowControl|MultiGate true true -1
    (:Out%200
      (Game|SpawnActorfromClass "/Game/BluePrints_Propios/BP_Pinches.BP_Pinches_C" (Math|Transform|MakeTransform (+ (Math|Vector|MakeVector (Math|Random|RandomFloatinRange 5e+02 1e+03) (Math|Random|RandomFloatinRange 5e+02 1e+03) 0.0) (Transformation|GetActorLocation))) "Undefined" "MultiplyWithRoot" 0 0))
    (:Out%201
      (Game|SpawnActorfromClass "/Game/BluePrints_Propios/BP_Heal.BP_Heal_C" (Math|Transform|MakeTransform (+ (Math|Vector|MakeVector (Math|Random|RandomFloatinRange 5e+02 1e+03) (Math|Random|RandomFloatinRange 5e+02 1e+03) 0.0) (Transformation|GetActorLocation))) "Undefined" "MultiplyWithRoot" 0 0))))

(fn ConstructionScript)