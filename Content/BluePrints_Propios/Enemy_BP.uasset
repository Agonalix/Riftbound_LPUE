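; Enemy actor Blueprint that drifts forward along its local X axis and can be destroyed by damage.
; It sets health to maximum on BeginPlay and steps a fixed offset after a per-frame Delay in Tick.
; ReceiveDMG subtracts health and, at the minimum, reports to BP_GM through WinCondition before destroying itself.
; Unconnected nodes for facing the player and spawning Bullet_E_BP never run.
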(event Custom|Receive%20DMG
  (params (DMG :type Float%20%28double-precision%29))
  (bind _output_get (Variables|Default|SetHP%20current (- (Variables|Default|GetHP%20current) DMG)))
  (if (<= _output_get (Variables|Default|GetHP%20Min))
    (bind _asbp_gm (Utilities|Casting|CastToBP_GM (Game|GetGameMode)))
    (Default|WinCondition _asbp_gm 1e+01)
    (Actor|DestroyActor)))

(event EventBeginPlay
  (Variables|Default|SetHP%20current (Variables|Default|GetHP%20Max)))

(event Collision|EventActorBeginOverlap
  (params (OtherActor :type Actor%20Object%20Reference)))

(event EventTick
  (params (DeltaSeconds :type Float%20%28single-precision%29))
  (Utilities|FlowControl|Delay DeltaSeconds)
  (Transformation|AddActorLocalOffset "5.000000,0.000000,0.000000" false false))

(fn ConstructionScript)