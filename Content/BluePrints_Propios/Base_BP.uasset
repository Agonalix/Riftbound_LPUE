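; Base actor that flags itself destroyed and reports a lose condition, apparently the structure the player must protect.
; Any overlap on its Box or any call to the damage event sets BaseDestroy, without checking HP or damage amount.
; LoseCon is called only if the overlapping or damaged actor itself casts to BP_GM.
; Tick resets HPCurrent to HPMax every frame.
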(event OnComponentBeginOverlap(Box)
  (params (OverlappedComponent :type Primitive%20Component%20Object%20Reference) (OtherActor :type Actor%20Object%20Reference) (OtherComp :type Primitive%20Component%20Object%20Reference) (OtherBodyIndex :type Integer) (bFromSweep :type Boolean) (SweepResult :type Hit%20Result%20Structure%20%28by%20ref%29))
  (Variables|Default|SetBaseDestroy true)
  (bind _asbp_gm (Utilities|Casting|CastToBP_GM OtherActor))
  (Default|LoseCon _asbp_gm (Variables|Default|GetBaseDestroy)))

(event Custom|OnTakeAnyDamage_Event
  (params (DamagedActor :type Actor%20Object%20Reference) (Damage :type Float%20%28single-precision%29) (DamageType :type Damage%20Type%20Object%20Reference) (InstigatedBy :type Controller%20Object%20Reference) (DamageCauser :type Actor%20Object%20Reference))
  (Variables|Default|SetBaseDestroy true)
  (bind _asbp_gm (Utilities|Casting|CastToBP_GM DamagedActor))
  (Default|LoseCon _asbp_gm (Variables|Default|GetBaseDestroy)))

(event EventBeginPlay)

(event Collision|EventActorBeginOverlap
  (params (OtherActor :type Actor%20Object%20Reference)))

(event EventTick
  (params (DeltaSeconds :type Float%20%28single-precision%29))
  (Variables|Default|SetHPCurrent (Variables|Default|GetHPMax)))

(fn ConstructionScript)