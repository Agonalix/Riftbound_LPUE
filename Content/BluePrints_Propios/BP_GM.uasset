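; Game manager Blueprint that tracks the score and decides when the game is won or lost.
; WinCondition adds incoming points to the current score and, once it reaches the WinCon threshold, opens the Victory level.
; LoseCon opens the Lose level when passed a true flag; both outcomes also print a debug string.
; ShipCount is an empty stub, and BeginPlay, Tick and the construction script do nothing.
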(event Custom|WinCondition
  (params (Puntos :type Float%20%28double-precision%29))
  ;[0.15 0.15 0.15 0.5] Win
  (Variables|Default|SetPuntaje%20Actual (+ (Variables|Default|GetPuntaje%20Actual) Puntos))
  (if (>= (Variables|Default|GetPuntaje%20Actual) (Variables|Default|GetWinCon))
    (Game|OpenLevel(byName) "Victory")
    (Development|PrintString "Ganaste maestro")))

(event Custom|Ship%20Count)

(event Custom|LoseCon
  (params (Lose :type Boolean))
  ;[0.15 0.15 0.15 0.5] Lose
  (if Lose
    (Game|OpenLevel(byName) "Lose")
    (Development|PrintString "BRUNO!!")))

(event EventBeginPlay)

(event EventTick
  (params (DeltaSeconds :type Float%20%28single-precision%29)))

(fn ConstructionScript)