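; BP_EnemyShip is an enemy ship that takes damage and destroys itself when its health runs out.
; Health resets to maximum on BeginPlay, and the ReceiveDMG event subtracts incoming damage until it reaches the minimum.
; After the destroy call, it casts OtherActor from the otherwise empty Collider hit event to BP_GM and, if that succeeds, decrements its Ships count.
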(event OnComponentHit(Collider)
  (params (HitComponent :type Primitive%20Component%20Object%20Reference) (OtherActor :type Actor%20Object%20Reference) (OtherComp :type Primitive%20Component%20Object%20Reference) (NormalImpulse :type Vector :default "0, 0, 0") (Hit :type Hit%20Result%20Structure%20%28by%20ref%29)))

(event Custom|Receive%20DMG
  (params (DMG :type Float%20%28double-precision%29))
  (bind _output_get (Variables|Default|SetHP%20Current (- (Variables|Default|GetHP%20Current) DMG)))
  (if (<= _output_get (Variables|Default|GetHP%20Min))
    (Actor|DestroyActor)
    (bind _asbp_gm (Utilities|Casting|CastToBP_GM (stale OnComponentHit(Collider) OtherActor)))
    (Variables|/Game/BluePrints_Propios/BP_GM.BP_GM_C|SetShips _asbp_gm (- (Variables|/Game/BluePrints_Propios/BP_GM.BP_GM_C|GetShips _asbp_gm) 1.0))))

(event EventBeginPlay
  (Variables|Default|SetHP%20Current (Variables|Default|GetHP%20Max)))

(event Collision|EventActorBeginOverlap
  (params (OtherActor :type Actor%20Object%20Reference)))

(event EventTick
  (params (DeltaSeconds :type Float%20%28single-precision%29)))

(fn ConstructionScript)