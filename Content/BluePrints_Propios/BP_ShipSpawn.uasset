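; BP_ShipSpawn is a spawn point actor that creates BP_EnemyShip enemies at its own transform when no ships remain.
; Tick polls the Ships count on BP_GM and, at zero or below, waits on a Delay before firing ShipSpawn, which also clears WaveInt.
; After spawning, it rechecks the count and calls WaveManager on BP_GM, found via GetActorOfClass, if at least two ships exist.
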(event Custom|ShipSpawn
  (Game|SpawnActorfromClass "/Game/BluePrints_Propios/BP_EnemyShip.BP_EnemyShip_C" (Transformation|GetActorTransform) "Undefined" "MultiplyWithRoot" 0 0)
  (Variables|Default|SetWaveInt false))

(event EventBeginPlay)

(event Collision|EventActorBeginOverlap
  (params (OtherActor :type Actor%20Object%20Reference)))

(event EventTick
  (params (DeltaSeconds :type Float%20%28single-precision%29))
  (bind _asbp_gm (Utilities|Casting|CastToBP_GM (Game|GetGameMode)))
  (if (<= (Variables|/Game/BluePrints_Propios/BP_GM.BP_GM_C|GetShips _asbp_gm) 0.0)
    (Utilities|FlowControl|Delay 1e+01)
    (CallFunction|ShipSpawn)
    (bind _asbp_gm_2 (Utilities|Casting|CastToBP_GM (Game|GetGameMode)))
    (if (>= (Variables|/Game/BluePrints_Propios/BP_GM.BP_GM_C|GetShips _asbp_gm_2) 2.0)
      (bind _returnvalue (Actor|GetActorOfClass "/Game/BluePrints_Propios/BP_GM.BP_GM_C"))
      (Default|WaveManager _returnvalue))))

(fn ConstructionScript)