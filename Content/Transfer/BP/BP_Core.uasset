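; BP_Core is a core actor with health whose depletion kills the player character.
; Health starts at MaxHealth on BeginPlay, and a custom event with damage-style parameters subtracts damage, clamped between zero and the maximum.
; At zero health it finds BP_ThirdPersonCharacter by class lookup and calls Die on it.
; The ApplyDamage function is an empty stub.
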(event Custom|CustomEvent
  (params (Damage :type Float%20%28single-precision%29) (DamageType :type Damage%20Type%20Object%20Reference) (InstigatedBy :type Controller%20Object%20Reference) (DamageCauser :type Actor%20Object%20Reference))
  (bind _output_get (Variables|Default|SetHealth (Math|Float|Clamp(Float) (- (Variables|Default|GetHealth) Damage) 0.0 (Variables|Default|GetMaxHealth))))
  (if (<= _output_get 0.0)
    (bind _returnvalue (Actor|GetActorOfClass "/Game/ThirdPerson/Blueprints/BP_ThirdPersonCharacter.BP_ThirdPersonCharacter_C"))
    (Default|Die _returnvalue)))

(event Collision|EventActorBeginOverlap
  (params (OtherActor :type Actor%20Object%20Reference)))

(event EventTick
  (params (DeltaSeconds :type Float%20%28single-precision%29)))

(event EventBeginPlay
  (Variables|Default|SetHealth (Variables|Default|GetMaxHealth)))

(fn ConstructionScript)

(fn ApplyDamage)